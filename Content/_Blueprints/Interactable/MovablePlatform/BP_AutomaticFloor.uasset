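; BP_AutomaticFloor is a moving platform that travels vertically back and forth on its own from BeginPlay.
; IsMoveDown selects the direction, and each direction has its own random range for the travel Distance, rolled once at start.
; The MovePlatform timeline scales its track by Distance to set the Cube's relative Z location.
; Its Finished pin feeds back into a FlipFlop that alternates Play and Reverse, looping the motion endlessly.
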(event `self.ReceiveBeginPlay`
  (`parent.ReceiveBeginPlay`)
  (if (`self.IsMoveDown`)
    (set `self.Distance` (* (`KismetMathLibrary.RandomFloatInRange` 1800.0 2500.0) -1.0))
    (`self.Move`)
    (else
      (set `self.Distance` (`KismetMathLibrary.RandomFloatInRange` 1000.0 10000.0))
      (`self.Move`))))

(event `Move`
  (`/Engine/EditorBlueprintResources/StandardMacros.FlipFlop` :!label _label
    (:`A`
      (bind (_direction _newtrack_1) (`Timeline|MovePlatform` :!label _label_2)
        (:`Update`
          (`SceneComponent.K2_SetRelativeLocation` (`self.Cube`) (`KismetMathLibrary.MakeVector` 0.0 0.0 (* _newtrack_1 (`self.Distance`))) false false))
        (:`Finished`
          (goto _label))))
    (:`B`
      (goto _label_2 :!via `Reverse`))))

(fn `UserConstructionScript`
  (`parent.UserConstructionScript`))