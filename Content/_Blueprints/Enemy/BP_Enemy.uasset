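; BP_Enemy is an enemy that chases and shoots at the player character when it sees one.
; PawnSensing sightings of BP_NewThirdPersonCharacter snap the enemy's rotation toward the target and start an AI MoveTo on it.
; The same sighting spawns a BP_EnemyBullet at BulletPosition, rate-limited by the ShootDelay flag and a Delay.
; The Shoot event is an empty stub.
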(event `Shoot`)

(event `self.PawnSensing.OnSeePawn`
  (params (Pawn :type "Pawn Object Reference"))
  (bind _asbp_new_third_person_character (cast `/Game/_Blueprints/ThirdPerson/Blueprints/BP_NewThirdPersonCharacter` Pawn))
  (`|ExecutionSequence`
    (:`then_0`
      (`self.K2_SetActorRotation` (`KismetMathLibrary.FindLookAtRotation` (`self.K2_GetActorLocation`) (`self.K2_GetActorLocation` _asbp_new_third_person_character)))
      (`|AIMoveTo` self (0.0 0.0 0.0) _asbp_new_third_person_character))
    (:`then_1`
      (if (`self.ShootDelay`)
        (`|SpawnActorFromClass` "/Game/_Blueprints/Enemy/BP_EnemyBullet.BP_EnemyBullet_C" (`SceneComponent.K2_GetComponentToWorld` (`self.BulletPosition`)) "Undefined" "MultiplyWithRoot" null null)
        (set `self.ShootDelay` false)
        (`KismetSystemLibrary.Delay` (`self.Delay Duration`))
        (set `self.ShootDelay` true)))))

(fn `UserConstructionScript`)