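; BP_Armor2 is an interactable armor item that changes the player character's armor.
; On Interact, it casts player character 0 to BP_NewThirdPersonCharacter, passes its ArmorColor to ArmorChange, then calls InteractItem.
; PickUpItem returns an empty string, and the BeginPlay, overlap and Tick events are unused.
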(event `/Game/_Blueprints/Inventory/BPI_PickUp.Interact`
  (bind _asbp_new_third_person_character (cast `/Game/_Blueprints/ThirdPerson/Blueprints/BP_NewThirdPersonCharacter` (`GameplayStatics.GetPlayerCharacter` 0)))
  (`/Game/_Blueprints/ThirdPerson/Blueprints/BP_NewThirdPersonCharacter.ArmorChange` _asbp_new_third_person_character (`self.ArmorColor`))
  (`self.InteractItem`))

(fn `PickUpItem`
  (returns (Item :type String))
  (return ""))

(fn `UserConstructionScript`
  (`parent.UserConstructionScript`))