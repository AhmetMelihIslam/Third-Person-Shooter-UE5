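; BP_Score is a score-keeping Blueprint that tracks how many enemies have been killed and how many remain.
; EnemyKill increments the kill count and calls EnemyDecrease to lower the remaining count, while EnemyIncrease raises it.
; It only holds counters behind these functions, with no active event logic, so changes depend on external callers.
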(fn `EnemyDecrease`
  (set `self.RemaningEnemyCount` (- (`self.RemaningEnemyCount`) 1)))

(fn `EnemyIncrease`
  (set `self.RemaningEnemyCount` (+ (`self.RemaningEnemyCount`) 1)))

(fn `EnemyKill`
  (set `self.EnemyKillCount` (+ (`self.EnemyKillCount`) 1))
  (`self.EnemyDecrease`))

(fn `UserConstructionScript`)