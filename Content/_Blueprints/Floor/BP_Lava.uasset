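; BP_Lava is a lava hazard that damages the third-person player character on contact and makes it jump.
; Box overlap enters a DoOnce that applies the damage, triggers the jump and sets IsOnPlayer.
; While that flag is set, Tick runs a short Delay into a FlipFlop that alternately resets and re-enters the DoOnce, repeating the hit.
; The character leaving the box clears the flag.
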(event `self.ReceiveTick`
  (params (DeltaSeconds :type "Float (single-precision)"))
  (`parent.ReceiveTick` DeltaSeconds)
  (if (`self.IsOnPlayer`)
    (`KismetSystemLibrary.Delay` 0.5)
    (`/Engine/EditorBlueprintResources/StandardMacros.FlipFlop`
      (:`A`
        (goto _label :!via `Reset`))
      (:`B`
        (`/Engine/EditorBlueprintResources/StandardMacros.DoOnce` false :!label _label
          (:`Completed`
            (bind _asbp_new_third_person_character (cast `/Game/_Blueprints/ThirdPerson/Blueprints/BP_NewThirdPersonCharacter` (stale `self.Box.OnComponentBeginOverlap` OtherActor)))
            (`/Game/_Blueprints/ThirdPerson/Blueprints/BP_NewThirdPersonCharacter.TakeDamage` _asbp_new_third_person_character 10.0)
            (`/Engine/EditorBlueprintResources/StandardMacros.IsValid` _asbp_new_third_person_character
              (:`Is Valid`
                (`Character.Jump` _asbp_new_third_person_character)
                (set `self.IsOnPlayer` true)))))))))

(event `self.Box.OnComponentBeginOverlap`
  (params (OverlappedComponent :type "PrimitiveComponent Object Reference") (OtherActor :type "Actor Object Reference") (OtherComp :type "PrimitiveComponent Object Reference") (OtherBodyIndex :type Integer) (bFromSweep :type Boolean) (SweepResult :type "HitResult Structure (by ref)"))
  (goto _label))

(event `self.Box.OnComponentEndOverlap`
  (params (OverlappedComponent :type "PrimitiveComponent Object Reference") (OtherActor :type "Actor Object Reference") (OtherComp :type "PrimitiveComponent Object Reference") (OtherBodyIndex :type Integer))
  (cast `/Game/_Blueprints/ThirdPerson/Blueprints/BP_NewThirdPersonCharacter` OtherActor)
  (set `self.IsOnPlayer` false))

(fn `UserConstructionScript`
  (`parent.UserConstructionScript`))